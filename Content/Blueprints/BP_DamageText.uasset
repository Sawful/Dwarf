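; BP_DamageText is a short-lived floating text actor, named for showing damage numbers.
; On BeginPlay a timer destroys the actor after half a second.
; Each tick moves its TextRender component upward at a speed scaled by a random factor re-rolled every frame, so the rise is slightly uneven.
; The file does not set the text itself.
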(event Custom|LifetimeEnd
  (Actor|DestroyActor))

(event EventBeginPlay
  (Utilities|Time|SetTimerbyEvent (delegate Custom|LifetimeEnd) 0.5))

(event EventTick
  (params (DeltaSeconds :type Float%20%28single-precision%29))
  (Transformation|AddRelativeLocation (Variables|Default|GetTextRender) (* (* (* DeltaSeconds 75.0) (Math|Random|RandomFloatinRange 1.0 2.5)) (Math|Vector|VectorUp)) false false))

(fn ConstructionScript)